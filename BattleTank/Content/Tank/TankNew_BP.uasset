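; Player-controllable tank Blueprint that routes input to aiming and movement components and carries a health bar widget.
; BeginPlay hands the barrel and turret to TankAiming, the tracks to TankMovement, and a self reference to the health bar.
; Aim axes rotate an azimuth gimbal and spring arm, while movement axes pass intent to TankMovement and Fire calls TankAiming.
; A swap input toggles the first- and third-person cameras.
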(event `self.ReceiveBeginPlay`
  (`TankAimingComponent.Initialise` (`self.TankAiming`) (`self.Barrel`) (`self.Turret`))
  (`TankMovementComponent.Initialise` (`self.TankMovement`) (`self.LeftTrack`) (`self.RightTrack`))
  (`self.InitialiseHealthBarWidget`))

(event `InputAction|Fire`
  (params (Key :type "Key Structure"))
  ;[1 1 1] Control Inputs
  (:`Pressed`
    (`TankAimingComponent.Fire` (`self.TankAiming`))))

(event `InputAxis|AimAzimuth`
  (params (AxisValue :type "Float (single-precision)"))
  ;[1 1 1] Aim Input Axis
  (`SceneComponent.K2_AddLocalRotation` (`self.AzimuthGimbal`) (`KismetMathLibrary.MakeRotator` 0.0 0.0 AxisValue) false false))

(event `InputAxis|Move Forward`
  (params (AxisValue :type "Float (single-precision)"))
  ;[1 1 1] Control Inputs
  (`TankMovementComponent.IntendMoveForward` (`self.TankMovement`) AxisValue))

(event `InputAxis|AimElevation`
  (params (AxisValue :type "Float (single-precision)"))
  ;[1 1 1] Aim Input Axis
  (`SceneComponent.K2_AddLocalRotation` (`self.SpringArm`) (`KismetMathLibrary.MakeRotator` 0.0 AxisValue) false false))

(event `InputAxis|Turn Right`
  (params (AxisValue :type "Float (single-precision)"))
  ;[1 1 1] Control Inputs
  (`TankMovementComponent.IntendTurnRight` (`self.TankMovement`) AxisValue))

(event `InputAction|SwapCameras`
  (params (Key :type "Key Structure"))
  ;[1 1 1] Camera Swapping
  (:`Pressed`
    (`ActorComponent.ToggleActive` (`self.FirstPersonCam`))
    (`ActorComponent.ToggleActive` (`self.ThirdPersonCam`))))

(fn `InitialiseHealthBarWidget`
  (bind _ashealth_bar (cast `/Game/UI/HealthBar` (`WidgetComponent.GetUserWidgetObject` (`self.Widget`))))
  (set `/Game/UI/HealthBar.Tank Reference` self _ashealth_bar)
  (return))

(fn `UserConstructionScript`)